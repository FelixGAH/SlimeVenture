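; A SlimeVenture actor that the player's SideScrollerCharacter can carry or move by attaching it to itself.
; Box overlap events track whether the character is in range.
; While in range with the character's AttachObejct flag set, Tick repeatedly snap-attaches the actor to the player and offsets it along Y.
; Tick detaches it once that flag clears, though MoveObject is never reset, so detaching repeats every such frame.
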(event OnComponentBeginOverlap(Box)
  (params (OverlappedComponent :type Primitive%20Component%20Object%20Reference) (OtherActor :type Actor%20Object%20Reference) (OtherComp :type Primitive%20Component%20Object%20Reference) (OtherBodyIndex :type Integer) (bFromSweep :type Boolean) (SweepResult :type Hit%20Result%20Structure%20%28by%20ref%29))
  (Utilities|Casting|CastToSideScrollerCharacter OtherActor)
  (bind _output_get (Variables|Default|SetOverlapp true)))

(event OnComponentEndOverlap(Box)
  (params (OverlappedComponent :type Primitive%20Component%20Object%20Reference) (OtherActor :type Actor%20Object%20Reference) (OtherComp :type Primitive%20Component%20Object%20Reference) (OtherBodyIndex :type Integer))
  (Utilities|Casting|CastToSideScrollerCharacter OtherActor)
  (Variables|Default|SetOverlapp false))

(event EventBeginPlay)

(event Collision|EventActorBeginOverlap
  (params (OtherActor :type Actor%20Object%20Reference)))

(event EventTick
  (params (DeltaSeconds :type Float%20%28single-precision%29))
  (bind _returnvalue (Game|GetPlayerCharacter 0))
  (Utilities|FlowControl|Sequence
    (:then_0
      (if (stale OnComponentBeginOverlap(Box) _output_get)
        (bind _asside_scroller_character (Utilities|Casting|CastToSideScrollerCharacter _returnvalue))
        (if (Variables|/Game/SideScrollerBP/Blueprints/SideScrollerCharacter.SideScrollerCharacter_C|GetAttachObejct _asside_scroller_character)
          (Variables|Default|SetMoveObject true)
          (Class|Actor|AttachRootComponenttoActor _returnvalue "None" "SnapToTarget" true)
          (Transformation|AddActorWorldOffset "0.000000,20.000000, 0"))))
    (:then_1
      (if (Variables|Default|GetMoveObject)
        (if (not (Variables|/Game/SideScrollerBP/Blueprints/SideScrollerCharacter.SideScrollerCharacter_C|GetAttachObejct _asside_scroller_character))
          (Class|Actor|DetachRootComponentfromParent true))))))

(fn ConstructionScript)