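; BP_Climb is a climb trigger actor that switches the side-scroller character in and out of its climb state.
; When its Box is overlapped by a character that is not climbing, it enables Climb and stores the character's location as WallPosition, but only above a speed threshold.
; An overlap by a character already climbing clears Climb and zeroes its rotation.
; The climbing movement itself is not handled here.
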(event OnComponentHit(Cube)
  (params (HitComponent :type Primitive%20Component%20Object%20Reference) (OtherActor :type Actor%20Object%20Reference) (OtherComp :type Primitive%20Component%20Object%20Reference) (NormalImpulse :type Vector :default "0, 0, 0") (Hit :type Hit%20Result%20Structure%20%28by%20ref%29)))

(event OnComponentBeginOverlap(Box)
  (params (OverlappedComponent :type Primitive%20Component%20Object%20Reference) (OtherActor :type Actor%20Object%20Reference) (OtherComp :type Primitive%20Component%20Object%20Reference) (OtherBodyIndex :type Integer) (bFromSweep :type Boolean) (SweepResult :type Hit%20Result%20Structure%20%28by%20ref%29))
  (bind _asside_scroller_character (Utilities|Casting|CastToSideScrollerCharacter OtherActor))
  (if (Variables|/Game/SideScrollerBP/Blueprints/SideScrollerCharacter.SideScrollerCharacter_C|GetClimb _asside_scroller_character)
    (Transformation|SetActorRotation _asside_scroller_character)
    (Variables|/Game/SideScrollerBP/Blueprints/SideScrollerCharacter.SideScrollerCharacter_C|SetClimb _asside_scroller_character false)
    (elif (> (Math|Vector|VectorLength (Transformation|GetVelocity _asside_scroller_character)) 5e+02)
      (Variables|/Game/SideScrollerBP/Blueprints/SideScrollerCharacter.SideScrollerCharacter_C|SetClimb _asside_scroller_character true)
      (Variables|/Game/SideScrollerBP/Blueprints/SideScrollerCharacter.SideScrollerCharacter_C|SetWallPosition _asside_scroller_character (Transformation|GetActorLocation _asside_scroller_character)))))

(event EventBeginPlay)

(event Collision|EventActorBeginOverlap
  (params (OtherActor :type Actor%20Object%20Reference)))

(event EventTick
  (params (DeltaSeconds :type Float%20%28single-precision%29)))

(fn ConstructionScript)